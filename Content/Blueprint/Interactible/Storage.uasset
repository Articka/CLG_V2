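; Interactible storage container that holds items and opens the storage UI for the Little_Girl_2D player when used.
; On BeginPlay it spawns an actor for each Container entry, flags it as stored and initializes it with the entry's count plus weight and sprite from the item DataTable.
; Table rows are found by class display name minus the "_C" suffix.
; Use passes the resulting Item list to the player's Storage; SetItem replaces it.
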(event EventBeginPlay
  (for _array_element (Variables|Default|GetContainer)
    (bind _returnvalue (Game|SpawnActorfromClass (.ItemToStore (Utilities|Struct|BreakStockage _array_element)) (Math|Transform|MakeTransform "0, 0, 0") "Undefined" 0 0))
    (Default|SetinStorage _returnvalue true)
    (bind _returnvalue_2 (Utilities|GetDataTableRow "/Game/Blueprint/Datatable/ItemInformation_-_Feuille_1.ItemInformation_-_Feuille_1" (Utilities|String|StringToName (Utilities|String|GetSubstring (Utilities|GetClassDisplayName (.ItemToStore (Utilities|Struct|BreakStockage _array_element))) 0 (Utilities|String|FindSubstring (Utilities|GetClassDisplayName (.ItemToStore (Utilities|Struct|BreakStockage _array_element))) "_C"))))
      (:then
        (Default|CreateNewItem _returnvalue (.Weight (Utilities|Struct|BreakItemInformation _returnvalue_2)) (.Sprite (Utilities|Struct|BreakItemInformation _returnvalue_2)) (.NumberOfItem (Utilities|Struct|BreakStockage _array_element)))
        (Utilities|Array|Add (Variables|Default|GetItem) _returnvalue)))))

(event EventUse
  (bind _aslittle_girl_2d (Utilities|Casting|CastToLittle_Girl_2D (Game|GetPlayerCharacter 0)))
  (Default|CreateStorage (Variables|/Game/Blueprint/LittleGirl/Little_Girl_2D.Little_Girl_2D_C|GetStorage _aslittle_girl_2d) (Variables|Default|GetItem))
  (Default|OpenStorage _aslittle_girl_2d self))

(fn ConstructionScript
  (|CallParentFunction))

(fn SetItem
  (params (NewItem :type Array%20of%20Actor%20Object%20References))
  (Variables|Default|SetItem NewItem)
  (return))