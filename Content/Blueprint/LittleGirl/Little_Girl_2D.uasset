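; Player character for a 2D point-and-click adventure starring a little girl who walks, inspects objects, collects items and talks.
; Left click sets an X-axis destination that Tick walks toward, flipping the sprite.
; Right click near an interactible opens an action menu; the chosen Look, Pick Up or Use runs once she reaches the object.
; It also manages inventory, storage and dialogue widgets, with Look text shown on a self-hiding text renderer.
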(event Custom|UnSetNewVisibilityOfTextPlayer
  ;[1 1 1] Action with interactible object
  ;;[1 1 1] Look action
  ;;;[1 1 1] Set and unset visibility of text renderer
  (Utilities|FlowControl|RetriggerableDelay 2.0)
  (CallFunction|SetVisibilityOfTextPlayer false))

(event Custom|Active%20action
  (params (Action :type String) (ObjectAction :type Actor%20Object%20Reference))
  ;[1 1 1] Action with interactible object
  ;;[1 1 1] When player as on object check selected action of player
  (switch string Action
    (:Look
      ;;[1 1 1] Look action
      ;;;[1 1 1] Set text renderer with look description
      (CallFunction|SetTextPlayer ObjectAction)
      ;;;[1 1 1] Set and unset visibility of text renderer
      (CallFunction|SetVisibilityOfTextPlayer true))
    (:Pick%20up
      ;;[1 1 1] PickUp Item
      (bind _asitem (Utilities|Casting|CastToItem ObjectAction))
      (Default|PickUp _asitem (Variables|Default|GetInventory)))
    (:Use
      ;;[1 1 1] Using interactible actor
      (bind _asinteractible (Utilities|Casting|CastToInteractible ObjectAction))
      (Default|Use _asinteractible))))

(event Custom|Talk
  (params (SetTalk :type String))
  (bind _talk_hud (Variables|Default|GetTalk_HUD))
  (Variables|Default|SetisTalking true)
  (Default|SetTalk _talk_hud SetTalk)
  (UserInterface|Viewport|AddtoViewport _talk_hud 0))

(event Custom|RemoveTalk
  (Widget|RemovefromParent (Variables|Default|GetTalk_HUD))
  (Variables|Default|SetisTalking false))

(event Custom|OpenStorage
  (params (RefOfStockage :type Object%20Object%20Reference))
  ;[1 1 1] Open stockage
  (Variables|Default|SetStorage_Ref RefOfStockage)
  (if (Variables|Default|GetinInventory)
    (Variables|Default|SetinInventory false)
    (else
      (Variables|Default|SetinInventory true)))
  (if (Variables|Default|GetinInventory)
    (UserInterface|Viewport|AddtoViewport (Variables|Default|GetInventory_HUD) 0)))

(event EventTick
  (params (DeltaSeconds :type Float%20%28single-precision%29))
  (bind _littlegirl (Variables|Default|GetLittleGirl))
  (bind _littlegirl_2 (Variables|Default|GetLittleGirl))
  (bind _relativerotation (Variables|/Script/Engine.SceneComponent|GetRelativeRotation _littlegirl))
  ;[1 0 0.05021] Event tick
  (Utilities|FlowControl|Sequence
    (:then_0
      ;;[1 1 1] Test destination, if is equal as 0, player don't move
      (if (not (Math|Vector|Equal(Vector) (Variables|Default|GetDestination) "0, 0, 0" 1.0))
        ;;[1 1 1] Check if the player move left or right
        (if (<= (.x (Transformation|GetActorLocation)) (.x (Variables|Default|GetDestination)))
          ;;[1 1 1] Move to destination
          (Pawn|Input|AddMovementInput (Math|Vector|MakeVector (.x (Variables|Default|GetDestination)) 0.0 0.0) 1.0 false)
          ;;[1 1 1] Rotate sprite
          (if (Math|Rotator|Equal(Rotator) _relativerotation "0,180.000000, 0" 5.0)
            (CallFunction|RotateSprite _littlegirl_2))
          ;;[1 1 1] Reset destination
          (if (Math|Vector|Equal(Vector) (Math|Vector|MakeVector (.x (Transformation|GetActorLocation)) 0.0 0.0) (Math|Vector|MakeVector (.x (Variables|Default|GetDestination)) 0.0 0.0) 5.0)
            (Variables|Default|SetDestination "0, 0, 0" :!label _label))
          (else
            (Pawn|Input|AddMovementInput (Math|Vector|MakeVector (.x (Variables|Default|GetDestination)) 0.0 0.0) -1.0 false)
            (if (Math|Rotator|Equal(Rotator) _relativerotation "0, 0, 0" 5.0)
              (CallFunction|RotateSprite _littlegirl_2))
            (if (Math|Vector|Equal(Vector) (Math|Vector|MakeVector (.x (Transformation|GetActorLocation)) 0.0 0.0) (Math|Vector|MakeVector (.x (Variables|Default|GetDestination)) 0.0 0.0) 5.0)
              (goto _label))))))
    (:then_1
      ;;[1 1 1] Move to object
      (if (!= (Variables|Default|GetGoToObject_MoveTo) 0)
        (bind _change__ (CallFunction|MovetoObject self (Variables|Default|GetGoToObject_MoveTo) (Variables|Default|GetIsOnObject)))
        (if _change__
          (CallFunction|ActiveAction (Variables|Default|GetActionOfMenu) (Variables|Default|GetGoToObject_MoveTo))
          (Variables|Default|SetGoToObject_MoveTo 0))))))

(event EventBeginPlay
  ;[0 1 0.0602] Event begin play
  ;;[1 1 1] Create widget menu action
  (bind _returnvalue (UserInterface|CreateWidget "/Game/Blueprint/HUD/MenuAction/MenuAction.MenuAction_C"))
  (Variables|Default|SetMenuAction _returnvalue)
  ;;[1 1 1] Create inventory HUD
  (bind _returnvalue_2 (UserInterface|CreateWidget "/Game/Blueprint/HUD/Inventory/Inventory_HUD.Inventory_HUD_C"))
  (Variables|Default|SetInventory_HUD _returnvalue_2)
  ;;[1 1 1] Create Storage HUD
  (bind _returnvalue_3 (UserInterface|CreateWidget "/Game/Blueprint/HUD/Stockage/Storage_HUD.Storage_HUD_C"))
  (Variables|Default|SetStorage _returnvalue_3)
  ;;[1 1 1] Talk HUD
  (bind _returnvalue_4 (UserInterface|CreateWidget "/Game/Blueprint/HUD/Talk/Talk.Talk_C"))
  (Variables|Default|SetTalk_HUD _returnvalue_4))

(event Input|ActionEvents|InputAction2D_Left_MouseClic
  (params (Key :type Key%20Structure))
  ;[1 1 1] Event left mouse clic
  (:Pressed
    (if (not (Variables|Default|GetinInventory))
      (if (not (Variables|Default|GetisTalking))
        (if (not (Variables|Default|GetisInteracting))
          ;;[1 1 1] Reset go to
          (Variables|Default|SetGoToObject_MoveTo 0)
          ;;[1 1 1] Set destination for player
          (bind _output_get (Variables|Default|SetDestination (.WorldLocation (Game|Player|ConvertMouseLocationToWorldSpace (Game|GetPlayerController 0)))))
          (else
            ;;[1 1 1] Set Go to object
            ;;;[1 1 1] Set go to object with touch actor
            (Variables|Default|SetGoToObject_MoveTo (Variables|Default|GetTouchActor))
            ;;;[1 1 1] Get selectioned action
            (bind _action (Default|GetActionSelection (Variables|Default|GetMenuAction)))
            (Variables|Default|SetActionOfMenu _action)))
        (else
          (Default|ActiononText (Variables|Default|GetTalk_HUD)))))))

(event Input|ActionEvents|InputAction2D_Open-CloseInventory
  (params (Key :type Key%20Structure))
  (bind _inventory_hud (Variables|Default|GetInventory_HUD))
  ;[1 1 1] InventoryDisplay
  (:Pressed
    (if (not (Variables|Default|GetisTalking))
      (if (Variables|Default|GetinInventory)
        (Variables|Default|SetinInventory false)
        (else
          (Variables|Default|SetinInventory true)))
      (if (Variables|Default|GetinInventory)
        (UserInterface|Viewport|AddtoViewport _inventory_hud 0)
        (else
          (Widget|RemovefromParent _inventory_hud))))))

(event Input|ActionEvents|InputAction2D_MenuSelection_Down
  (params (Key :type Key%20Structure))
  ;[1 1 1] Event menu selection
  (:Pressed
    ;;[1 1 1] Set selection menu action
    (if (Variables|Default|GetisInteracting)
      (Default|SetUpDownMenuSelection (Variables|Default|GetMenuAction) "Down"))))

(event Input|ActionEvents|InputAction2D_MenuSelection_Up
  (params (Key :type Key%20Structure))
  ;[1 1 1] Event menu selection
  (:Pressed
    ;;[1 1 1] Set selection menu action
    (if (Variables|Default|GetisInteracting)
      (Default|SetUpDownMenuSelection (Variables|Default|GetMenuAction) "Up"))))

(event Input|ActionEvents|InputAction2D_Right_MouseClic
  (params (Key :type Key%20Structure))
  ;[1 1 1] Event right mouse clic
  (:Pressed
    (if (and (not (Variables|Default|GetinInventory)) (not (Variables|Default|GetisTalking)))
      ;;[1 1 1] Create menu action for player
      (if (Variables|Default|GetCanInteractible)
        (Variables|Default|SetisInteracting true)
        (UserInterface|Viewport|AddtoViewport (Variables|Default|GetMenuAction) 0)))))

(event Input|KeyboardEvents|K
  (params (Key :type Key%20Structure))
  (:Pressed
    (CallFunction|Talk "Test")))

(fn ConstructionScript)

(fn RemovefromParentMenuAction
  (Widget|RemovefromParent (Variables|Default|GetMenuAction))
  (Variables|Default|SetisInteracting false)
  (return))

(fn SetTextPlayer
  (params (ObjectAction :type Actor%20Object%20Reference))
  (bind _asinteractible (Utilities|Casting|CastToInteractible ObjectAction))
  (bind _looking_description (Default|Look _asinteractible))
  (Rendering|Components|TextRender|SetText (Variables|Default|GetTextPlayer) (Utilities|Text|ToText(String) _looking_description))
  (return))

(fn SetVisibilityOfTextPlayer
  (params (NewVisibility :type Boolean))
  (Rendering|SetVisibility (Variables|Default|GetTextPlayer) NewVisibility false)
  (if NewVisibility
    (CallFunction|UnSetNewVisibilityOfTextPlayer))
  (return))

(fn InventorySetInventory
  (params (NewInventory :type Inventory%20Structure))
  (bind _output_get (Variables|Default|SetInventory (Utilities|Struct|MakeInventory (.maximumofdifferentobject NewInventory) (.maximumofweight NewInventory) (.actualweight NewInventory) (.itemactor NewInventory))))
  (return _output_get))

(fn InventoryAddIteminInventory
  (params (ItemToAdd :type Actor%20Object%20Reference))
  (bind _returnvalue (Utilities|Array|Add (.itemactor (Variables|Default|GetInventory)) ItemToAdd))
  (return _returnvalue))

(fn InventorySetIteminInventory
  (params (Index :type Integer) (NewActorSet :type Actor%20Object%20Reference))
  (Utilities|Array|SetArrayElem (.itemactor (Variables|Default|GetInventory)) Index NewActorSet)
  (return))

(fn InventoryActioninInventory
  (params (RefOfActor :type Actor%20Object%20Reference) (Action :type Text))
  ;[1 1 1] Default = Use
  (switch string (Utilities|String|ToString(Text) Action)
    (:Default
      (bind _asitem (Utilities|Casting|CastToItem RefOfActor :!label _label))
      (Default|Use _asitem))
    (:Look
      (CallFunction|SetTextPlayer RefOfActor)
      (CallFunction|SetVisibilityOfTextPlayer true))
    (:Use
      (goto _label))
    (:Pick%20Up
      (bind _asitem_2 (Utilities|Casting|CastToItem RefOfActor))
      (if (Variables|/Game/Blueprint/Item/MotherClass/Item.Item_C|GetinStorage _asitem_2)
        (bind _asstorage (Utilities|Casting|CastToStorage (Variables|Default|GetIsOnObject)))
        (for _array_element (Variables|/Game/Blueprint/Interactible/Storage.Storage_C|GetItem _asstorage)
          (if (== _array_element _asitem_2)
            (Utilities|Array|RemoveItem (Variables|/Game/Blueprint/Interactible/Storage.Storage_C|GetItem _asstorage) _array_element)
            (Default|PickUp _asitem_2 (Variables|Default|GetInventory))))
        (else
          (Default|PickUp _asitem_2 (Variables|Default|GetInventory)))))))

(fn InventoryAddIteminInventoryNumber
  (params (ItemToAdd :type Actor%20Object%20Reference) (NumberOfItemTake :type Integer))
  (bind _returnvalue (Utilities|Array|Add (.itemactor (Variables|Default|GetInventory)) ItemToAdd))
  (return _returnvalue))