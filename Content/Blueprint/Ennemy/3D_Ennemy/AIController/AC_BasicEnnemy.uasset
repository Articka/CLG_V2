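; AI controller for the basic 3D enemy that reacts to seeing or losing the Little Girl player.
; On BeginPlay it sets up the BB_BasicEnnemy blackboard, seeds the GoToTP key and runs the basic enemy behavior tree.
; AI Perception updates for the Little Girl set the PlayerDetected blackboard key and call PlayerDetect on the controlled BasicEnnemy_3D pawn with the same state.
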(event OnTargetPerceptionUpdated(AIPerception)
  (params (Actor :type Actor%20Object%20Reference) (Stimulus :type AI%20Stimulus%20Structure))
  (bind _returnvalue (Utilities|Name|MakeLiteralName "PlayerDetected"))
  (bind _self self)
  (bind _blackboard (Variables|Default|GetBlackboard))
  (bind _returnvalue_2 (AI|GetAIController _self))
  (bind _returnvalue_3 (Pawn|GetControlledPawn _returnvalue_2))
  (Utilities|Casting|CastToLittle_Girl_3D Actor)
  (if (.bSuccessfullySensed (Utilities|Struct|BreakAIStimulus Stimulus))
    (AI|Components|Blackboard|SetValueasBool _blackboard _returnvalue true)
    (bind _asbasic_ennemy_3d (Utilities|Casting|CastToBasicEnnemy_3D _returnvalue_3))
    (Default|PlayerDetect _asbasic_ennemy_3d true)
    (else
      (AI|Components|Blackboard|SetValueasBool _blackboard _returnvalue false)
      (bind _asbasic_ennemy_3d_2 (Utilities|Casting|CastToBasicEnnemy_3D _returnvalue_3))
      (Default|PlayerDetect _asbasic_ennemy_3d_2 false))))

(event EventBeginPlay
  (bind _blackboardcomponent (Class|AIController|UseBlackboard "/Game/Blueprint/Ennemy/3D_Ennemy/BB/BB_BasicEnnemy.BB_BasicEnnemy"))
  (Class|BlackboardComponent|SetValueasInt _blackboardcomponent (Utilities|Name|MakeLiteralName "GoToTP") 2)
  (AI|RunBehaviorTree "/Game/Blueprint/Ennemy/3D_Ennemy/BT/BT_BasicEnnnemy.BT_BasicEnnnemy"))

(fn ConstructionScript)