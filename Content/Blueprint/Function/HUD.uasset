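; HUD function library for building inventory menu entries: item buttons, quantity labels and action lists.
; AddButton creates a ButtonItemInventory widget for an item, names it in French or English from a DataTable row keyed by GetSprite, and returns the item count.
; AddNumberOfItem adds an "x"-prefixed count label.
; GetAllAction splits an action string on underscores, keeping only segments terminated by an underscore.
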(fn AddButton
  (params (Actor_Item :type Actor%20Object%20Reference) (AddChild :type Panel%20Widget%20Object%20Reference) (AllButton :type Array%20of%20Button%20Item%20Inventory%20Object%20References))
  (bind _returnvalue (UserInterface|CreateWidget "/Game/Blueprint/HUD/Inventory/ButtonItemInventory.ButtonItemInventory_C"))
  (Default|SetRefOfActor _returnvalue Actor_Item)
  (Utilities|Array|Add AllButton _returnvalue)
  (bind _asitem (Utilities|Casting|CastToItem Actor_Item))
  (bind _returnvalue_2 (Default|GetSprite _asitem))
  (bind _returnvalue_3 (Utilities|GetDataTableRow "/Game/Blueprint/Datatable/MenuInteractObject_-_Feuille_1__11_.MenuInteractObject_-_Feuille_1__11_" (Utilities|String|StringToName _returnvalue_2))
    (:then
      (bind _aslittle_girl_gamemode__2d (Utilities|Casting|CastToLittle_Girl_Gamemode__2D (Game|GetGameMode)))
      (Default|SetNameOfItem _returnvalue (Utilities|String|StringToName _returnvalue_2))
      (switch Utilities|FlowControl|Switch|SwitchonLanguageOfTheGame (Variables|/Game/Blueprint/LittleGirl/Little_Girl_Gamemode__2D.Little_Girl_Gamemode__2D_C|GetLanguageOfTheGame _aslittle_girl_gamemode__2d)
        (:NewEnumerator0
          (Default|SetTextButton _returnvalue (Utilities|Text|ToText(String) (.NameOfObject_FR (Utilities|Struct|BreakMenuInteractObject _returnvalue_3)))))
        (:NewEnumerator1
          (Default|SetTextButton _returnvalue (Utilities|Text|ToText(String) (.NameOfObject_EN (Utilities|Struct|BreakMenuInteractObject _returnvalue_3))))))
      (Widget|Panel|AddChild AddChild _returnvalue)
      (return (Variables|/Game/Blueprint/Item/MotherClass/Item.Item_C|GetNumberOfItem _asitem)))))

(fn AddNumberOfItem
  (params (NumberOfItem :type Integer) (AllTextNumberItem :type Array%20of%20Child%20Text%20Object%20References) (ChildNumberOfItem :type Panel%20Widget%20Object%20Reference))
  ;[1 1 1] Set_Create number of item
  (bind _returnvalue (UserInterface|CreateWidget "/Game/Blueprint/HUD/Children/Child_Text.Child_Text_C"))
  (Utilities|Array|Add AllTextNumberItem _returnvalue)
  (Default|SetNewPadding _returnvalue 5.0)
  (Default|SetText _returnvalue (Utilities|String|Append "x" (Utilities|String|ToString(Integer) NumberOfItem)))
  (Widget|Panel|AddChild ChildNumberOfItem _returnvalue)
  (return))

(fn GetAllAction
  (params (Action :type String) (AllTextAction :type Array%20of%20Strings))
  (LocalVariables|SetNewActionName "")
  (for _array_element (Utilities|String|GetCharacterArrayfromString Action)
    (if (not (Utilities|Enum|Equal(Enum) _array_element "_"))
      (LocalVariables|SetNewActionName (Utilities|String|Append (LocalVariables|GetNewActionName) _array_element))
      (else
        (Utilities|Array|Add AllTextAction (LocalVariables|GetNewActionName))
        (LocalVariables|SetNewActionName "")))))