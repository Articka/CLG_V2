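; MoveToObject is a Blueprint function that walks a 2D Paper2D character along X toward a target object and reports arrival.
; Each call compares X positions, adds signed movement input to the instigator pawn using the target's world X as direction vector, and flips the flipbook sprite via RotateSprite when needed.
; Arrival means the target equals the IsOnObject input, with a location tolerance check gating movement.
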(fn MovetoObject
  (params (ForSelf :type Actor%20Object%20Reference) (ToObject :type Actor%20Object%20Reference) (IsOnObject :type Actor%20Object%20Reference))
  (bind _returnvalue (Transformation|GetActorLocation ToObject))
  (bind _returnvalue_2 (Transformation|GetActorLocation ToObject))
  (bind _returnvalue_3 (Actor|GetComponentbyClass ForSelf "/Script/Paper2D.PaperFlipbookComponent"))
  (bind _rootcomponent (Variables|/Script/Engine.Actor|GetRootComponent ForSelf))
  (bind _instigator (Variables|/Script/Engine.Actor|GetInstigator ForSelf))
  (bind _returnvalue_4 (Transformation|GetWorldLocation _rootcomponent))
  (bind _x (Math|Vector|BreakVector _returnvalue_2))
  (bind _relativerotation (Variables|/Script/Engine.SceneComponent|GetRelativeRotation _returnvalue_3))
  (bind _returnvalue_5 (Math|Vector|MakeVector _x 0.0 0.0))
  (if (== ToObject IsOnObject)
    (return 0 true true)
    (elif (Math|Vector|NotEqual(Vector) _returnvalue_4 _returnvalue 5.0)
      (if (>= (.X (Math|Vector|BreakVector _returnvalue_4)) (.X (Math|Vector|BreakVector _returnvalue)))
        (Pawn|Input|AddMovementInput _instigator _returnvalue_5 -1.0 false)
        ;[1 1 1] Rotate sprite
        (if (Math|Rotator|Equal(Rotator) _relativerotation "0, 0, 0" 5.0)
          (CallFunction|RotateSprite _returnvalue_3))
        (else
          (Pawn|Input|AddMovementInput _instigator _returnvalue_5 1.0 false)
          (if (Math|Rotator|Equal(Rotator) _relativerotation "0,180.000000, 0" 5.0)
            (CallFunction|RotateSprite _returnvalue_3))))
      (if (== ToObject IsOnObject)
        (return 0 true true)
        (else
          (return 0 false false))))))